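; BP_Level is a level-management Blueprint that sets the player's input mode and ramps up game speed over time.
; On BeginPlay it checks the level name, using UI-only input with a visible cursor for Map_MainMenu and game-only input otherwise.
; Every tick, in any level, UpdateGameSpeed raises GameSpeed by GameSpeedIncrement scaled by delta time, giving a steady, frame-rate-independent increase.
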(event Custom|UpdateGameSpeed
  (Variables|Default|SetgameSpeed (+ (Variables|Default|GetgameSpeed) (* (stale EventTick DeltaSeconds) (Variables|Default|GetgameSpeedIncrement)))))

(event EventBeginPlay
  (bind _returnvalue (Game|GetPlayerController 0))
  (bind _returnvalue_2 (Game|GetCurrentLevelName true))
  (if (Utilities|Enum|Equal(Enum) _returnvalue_2 "Map_MainMenu")
    (Input|SetInputModeUIOnly _returnvalue 0 "DoNotLock" false)
    (Variables|/Script/Engine.PlayerController|SetbShowMouseCursor _returnvalue true)
    (else
      (Input|SetInputModeGameOnly _returnvalue false))))

(event EventTick
  (params (DeltaSeconds :type Float%20%28single-precision%29))
  (CallFunction|UpdateGameSpeed))

(fn ConstructionScript)