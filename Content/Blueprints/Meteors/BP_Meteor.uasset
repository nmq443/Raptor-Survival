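; BP_Meteor is a meteor projectile that scales with the level's game speed and destroys itself on hitting the tile map.
; On BeginPlay it caches the BP_Level actor as its level controller.
; Every Tick multiplies the projectile movement's current InitialSpeed and MaxSpeed by the controller's GameSpeed, so the scaling compounds each frame.
; A Hitbox overlap with a PaperTileMapActor destroys the meteor.
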(event OnComponentBeginOverlap(Hitbox)
  (params (OverlappedComponent :type Primitive%20Component%20Object%20Reference) (OtherActor :type Actor%20Object%20Reference) (OtherComp :type Primitive%20Component%20Object%20Reference) (OtherBodyIndex :type Integer) (bFromSweep :type Boolean) (SweepResult :type Hit%20Result%20Structure%20%28by%20ref%29))
  (Utilities|Casting|CastToPaperTileMapActor OtherActor)
  (Actor|DestroyActor))

(event Custom|UpdateSpeed
  (bind _projectilemovement (Variables|Default|GetProjectileMovement))
  (bind _levelcontroller (Variables|Default|GetlevelController))
  (bind _gamespeed (Variables|/Game/Blueprints/System/BP_Level.BP_Level_C|GetgameSpeed _levelcontroller))
  (Variables|/Script/Engine.ProjectileMovementComponent|SetInitialSpeed _projectilemovement (* _gamespeed (Variables|/Script/Engine.ProjectileMovementComponent|GetInitialSpeed _projectilemovement)))
  (Variables|/Script/Engine.ProjectileMovementComponent|SetMaxSpeed _projectilemovement (* _gamespeed (Class|MovementComponent|GetMaxSpeed _projectilemovement))))

(event EventBeginPlay
  (bind _returnvalue (Actor|GetActorOfClass "/Game/Blueprints/System/BP_Level.BP_Level_C"))
  (Variables|Default|SetlevelController _returnvalue))

(event EventTick
  (params (DeltaSeconds :type Float%20%28single-precision%29))
  (CallFunction|UpdateSpeed))

(fn ConstructionScript)